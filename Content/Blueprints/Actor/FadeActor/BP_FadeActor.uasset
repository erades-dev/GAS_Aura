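; Static mesh actor that fades out and back in by driving a "Fade" material parameter through a timeline.
; Construction caches the original materials and builds dynamic instances from a separate fade material list.
; FadeOut swaps those instances onto the mesh and plays the timeline, while Fadein reverses it.
; When the timeline finishes at 1 or above, the original materials are restored; collision toggles are unconnected.
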(event `self.ReceiveBeginPlay`)

(event `/Game/Blueprints/Actor/FadeActor/BPI_Fade.FadeOut`
  (`self.SetMaterialsToDynamicInstances`)
  (bind (_direction _newtrack_0) (`Timeline|FadeTimeline` :!label _label)
    (:`Update`
      (for _array_element (`self.DynamicMaterials`)
        (`MaterialInstanceDynamic.SetScalarParameterValue` _array_element "Fade" _newtrack_0)))
    (:`Finished`
      (`self.FadeFinish` _newtrack_0))))

(event `/Game/Blueprints/Actor/FadeActor/BPI_Fade.FadeIn`
  (goto _label :!via `Reverse`))

(fn `FadeFinish`
  (params (InputPin :type "Float (single-precision)"))
  (if (>= InputPin 1.0)
    (`self.ResetMaterials`)
    (elif (<= InputPin 0.0)
      _)))

(fn `ResetMaterials`
  (for (_array_element _array_index) (`self.OriginalMaterials`)
    (`PrimitiveComponent.SetMaterial` (`self.StaticMesh`) _array_index _array_element)))

(fn `SetMaterialsToDynamicInstances`
  (for (_array_element _array_index) (`self.DynamicMaterials`)
    (`PrimitiveComponent.SetMaterial` (`self.StaticMesh`) _array_index _array_element)))

(fn `UserConstructionScript`
  (`|ExecutionSequence`
    (:`then_0`
      (set `self.OriginalMaterials` (`MeshComponent.GetMaterials` (`self.StaticMesh`))))
    (:`then_1`
      (`KismetArrayLibrary.Array_Clear` (`self.DynamicMaterials`)))
    (:`then_2`
      (for _array_element (`self.FadeMaterialInstances`)
        (bind _returnvalue (`KismetMaterialLibrary.CreateDynamicMaterialInstance` _array_element))
        (`KismetArrayLibrary.Array_Add` (`self.DynamicMaterials`) _returnvalue)))))