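; BP_EnemyBase is an enemy base Blueprint that handles attack facing and a dissolve effect.
; UpdateFacingTarget feeds a projectile target location into the Motion Warping "FacingTarget" warp target.
; StartDissolveTimeline waits briefly, then starts two timelines that drive the Dissolve scalar parameter on the first two supplied dynamic material instances.
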(event `CombatInterface.UpdateFacingTarget`
  (params (ProjectileTargetLocation :type "Vector Structure"))
  (`MotionWarpingComponent.AddOrUpdateWarpTargetFromLocation` (`self.MotionWarping`) "FacingTarget" ProjectileTargetLocation))

(event `self.StartDissolveTimeline`
  (params (DynamicMaterialInstance :type "Array of MaterialInstanceDynamic Object Reference (by ref)"))
  (`KismetSystemLibrary.Delay` 2.0)
  (`|ExecutionSequence`
    (:`then_0`
      (bind (_direction _value) (`Timeline|Dissolve0`)
        (:`Update`
          (`MaterialInstanceDynamic.SetScalarParameterValue` (`|GetArrayItem` DynamicMaterialInstance) "Dissolve" _value))))
    (:`then_1`
      (bind (_direction_2 _value_2) (`Timeline|Timeline`)
        (:`Update`
          (`MaterialInstanceDynamic.SetScalarParameterValue` (`|GetArrayItem` DynamicMaterialInstance 1) "Dissolve" _value_2))))))

(fn `UserConstructionScript`)