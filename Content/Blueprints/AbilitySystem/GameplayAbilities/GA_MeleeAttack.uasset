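; Gameplay ability for a melee attack that turns the avatar toward its combat target and damages enemies near the strike point.
; It plays a random tagged attack montage and waits for that montage's tag as a gameplay event.
; On the event, it sphere-queries live players around the tag's combat socket and damages non-friends, with debug spheres and prints.
; The ability ends when the montage completes, is interrupted or is cancelled.
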(event `self.K2_ActivateAbility`
  (bind _returnvalue (`self.GetAvatarActorFromActorInfo`))
  (bind _returnvalue_2 (`self.GetAvatarActorFromActorInfo`))
  (bind (_montage _montagetag) (break `TaggedMontage` (`self.TaggedMontage`)))
  (`|ExecutionSequence`
    (:`then_0`
      (bind _returnvalue_3 (message `CombatInterface.GetCombatTarget` _returnvalue_2))
      (message `CombatInterface.UpdateFacingTarget` _returnvalue_2 (`Actor.K2_GetActorLocation` _returnvalue_3)))
    (:`then_1`
      (bind _returnvalue_4 (message `CombatInterface.GetAttackMontages` (`self.GetAvatarActorFromActorInfo`)))
      (bind _output_get (set `self.TaggedMontage` (`self.GetRandomTaggedMontageFromArray` _returnvalue_4)))
      (`AbilityTask_PlayMontageAndWait.CreatePlayMontageAndWaitProxy` "None" (`.Montage` (break `TaggedMontage` _output_get)) 1.0 "None" false
        (:`then`
          (`AbilityTask_WaitGameplayEvent.WaitGameplayEvent` _montagetag null
            (:`EventReceived`
              (bind _returnvalue_5 (message `CombatInterface.GetCombatSocketLocation` _returnvalue _montagetag))
              (`KismetSystemLibrary.DrawDebugSphere` _returnvalue_5 45.0 12 (struct :`R` 1.0 :`G` 1.0 :`B` 1.0 :`A` 1.0) 0.1 1.0)
              (bind _outoverlappingactors (`AuraAbilitySystemLibrary.GetLifePlayersWithinRadius` self (`|MakeArray` _returnvalue) 45.0 _returnvalue_5))
              (for _array_element _outoverlappingactors
                (if (`AuraAbilitySystemLibrary.IsNotFriend` _array_element (`self.GetAvatarActorFromActorInfo`))
                  (`self.CauseDamage` _array_element)
                  (`KismetSystemLibrary.PrintString` (`KismetSystemLibrary.GetDisplayName` _array_element))
                  (`KismetSystemLibrary.DrawDebugSphere` (`Actor.K2_GetActorLocation` _array_element) 35.0 12 (struct :`R` 1.0 :`B` 0.083856 :`A` 1.0) 0.5))))))
        (:`OnCompleted`
          (`self.K2_EndAbility` :!label _label))
        (:`OnInterrupted`
          (goto _label))
        (:`OnCancelled`
          (goto _label))))))