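; Gameplay ability for a ranged attack that fires a projectile at the avatar's combat target.
; It turns the avatar toward the target and plays a random tagged montage.
; The montage tag's gameplay event spawns the projectile from the tagged socket toward the target's current location.
; A debug sphere marks activation, and the ability ends on a fixed delay without stopping the montage.
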(event `self.K2_ActivateAbility`
  (bind _returnvalue (`self.GetAvatarActorFromActorInfo`))
  (bind (_montage _montagetag _sockettag) (break `TaggedMontage` (`self.TaggedMontage`)))
  (`|ExecutionSequence`
    (:`then_0`
      (`KismetSystemLibrary.DrawDebugSphere` (`Actor.K2_GetActorLocation` (`self.GetAvatarActorFromActorInfo`)) 100.0 12 (struct :`R` 1.0 :`G` 1.0 :`B` 1.0 :`A` 1.0) 1.0))
    (:`then_1`
      (bind _returnvalue_2 (message `CombatInterface.GetCombatTarget` _returnvalue))
      (message `CombatInterface.UpdateFacingTarget` _returnvalue (`Actor.K2_GetActorLocation` _returnvalue_2)))
    (:`then_2`
      (bind _returnvalue_3 (message `CombatInterface.GetAttackMontages` (`self.GetAvatarActorFromActorInfo`)))
      (bind _output_get (set `self.TaggedMontage` (`self.GetRandomTaggedMontageFromArray` _returnvalue_3)))
      (`AbilityTask_PlayMontageAndWait.CreatePlayMontageAndWaitProxy` "None" (`.Montage` (break `TaggedMontage` _output_get)) 1.0 "None" false
        (:`then`
          (`AbilityTask_WaitGameplayEvent.WaitGameplayEvent` _montagetag null true
            (:`EventReceived`
              (bind _returnvalue_4 (message `CombatInterface.GetCombatTarget` (`self.GetAvatarActorFromActorInfo`)))
              (`self.SpawnProjectile` (`Actor.K2_GetActorLocation` _returnvalue_4) _sockettag))))))
    (:`then_3`
      (`KismetSystemLibrary.Delay` 1.0)
      (`self.K2_EndAbility`))))